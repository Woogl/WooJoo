(event `Server_Action`
  (bind _asbp_woogle_game_mode (cast `/Game/Woogle/BP_WoogleGameMode` (`GameplayStatics.GetGameMode`)))
  (`/Game/Woogle/BP_WoogleGameMode.CycleTurns` _asbp_woogle_game_mode))

(event `self.ReceiveBeginPlay`
  ;[0 0 0] Setup
  (bind _returnvalue (`|AddComponentByClass` (`self.GetOwner`) "/Game/Blueprints/Components/BP_DisplayerManager.BP_DisplayerManager_C" "/Game/Blueprints/BP_Displayer.BP_Displayer_C" false null))
  (set `self.DisplayerManager_Turn` _returnvalue))

(event `OnStartBoardGame`
  (if (`Controller.IsLocalController` (`GameplayStatics.GetPlayerController` 0))
    (`/Game/Blueprints/Components/BP_DisplayerManager.CreateDisplayer` (`self.DisplayerManager_Turn`) (select `bool` (`self.IsMyTurn`) :`false` "WAITING" :`true` "YOUR TURN" :!type "Text") (`self.GetRightUIPosition`))))

(event `Key|SpaceBar`
  (params (Key :type "Key Structure"))
  ;[1 1 1] Input Test
  (:`Pressed`
    (if (`self.IsMyTurn`)
      (`self.HandleSpaceBar`))))

(event `Key|Enter`
  (params (Key :type "Key Structure"))
  ;[1 1 1] Input Test
  (:`Pressed`
    (bind _asbp_woogle_game_mode (cast `/Game/Woogle/BP_WoogleGameMode` (`GameplayStatics.GetGameMode`)))
    (`/Game/Woogle/BP_WoogleGameMode.LetsStart` _asbp_woogle_game_mode)))

(event `OnStartTurn`
  (set `self.IsMyTurn` true)
  (`/Game/Blueprints/Components/BP_DisplayerManager.EditDisplayer` (`self.DisplayerManager_Turn`) "YOUR TURN"))

(event `OnEndTurn`
  (set `self.IsMyTurn` false)
  (`/Game/Blueprints/Components/BP_DisplayerManager.EditDisplayer` (`self.DisplayerManager_Turn`) "WAITING"))

(fn `HandleSpaceBar`
  (`self.Server_Action`))