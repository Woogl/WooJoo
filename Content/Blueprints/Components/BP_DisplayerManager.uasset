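; Component that manages a single displayer actor showing a text message in the world, with create, edit and delete events.
; A ShouldReplicates flag routes each call to Server or Client events, with create and edit playing a 2D sound, multicast when replicated.
; Creation moves an existing displayer or spawns one turned toward the owner with zero pitch.
; Server deletion falls back to finding any actor of the displayer class when the stored reference is invalid.
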(event `Server_CreateDisplayer`
  (params (InText :type Text) (DisplayerLocation :type "Vector Structure"))
  (bind (_returnvalue_roll _returnvalue_pitch _returnvalue_yaw) (`KismetMathLibrary.BreakRotator` (`KismetMathLibrary.FindLookAtRotation` DisplayerLocation (`Actor.K2_GetActorLocation` (`self.GetOwner`)))))
  (`/Engine/EditorBlueprintResources/StandardMacros.IsValid` (`self.DisplayerActor`)
    (:`Is Valid`
      (`Actor.K2_SetActorLocation` (`self.DisplayerActor`) DisplayerLocation false true)
      (message `/Game/Blueprints/Interfaces/BPI_Displayer.ChangeText` (`self.DisplayerActor`) InText))
    (:`Is Not Valid`
      (bind _returnvalue (`|SpawnActorFromClass` (`self.DisplayerClass`) (`KismetMathLibrary.MakeTransform` DisplayerLocation (`KismetMathLibrary.MakeRotator` _returnvalue_roll 0.0 _returnvalue_yaw)) "AlwaysSpawn" "OverrideRootScale" null (`self.ShouldReplicates`) (`GameplayStatics.GetPlayerPawn` 0)))
      (bind _output_get (set `self.DisplayerActor` _returnvalue))
      (message `/Game/Blueprints/Interfaces/BPI_Displayer.ChangeText` _output_get InText))))

(event `Client_CreateDisplayer`
  (params (TextToShow :type Text) (DisplayerLocation :type "Vector Structure"))
  (bind (_returnvalue_roll _returnvalue_pitch _returnvalue_yaw) (`KismetMathLibrary.BreakRotator` (`KismetMathLibrary.FindLookAtRotation` DisplayerLocation (`Actor.K2_GetActorLocation` (`self.GetOwner`)))))
  (`/Engine/EditorBlueprintResources/StandardMacros.IsValid` (`self.DisplayerActor`)
    (:`Is Valid`
      (`Actor.K2_SetActorLocation` (`self.DisplayerActor`) DisplayerLocation false true)
      (message `/Game/Blueprints/Interfaces/BPI_Displayer.ChangeText` (`self.DisplayerActor`) TextToShow))
    (:`Is Not Valid`
      (bind _returnvalue (`|SpawnActorFromClass` (`self.DisplayerClass`) (`KismetMathLibrary.MakeTransform` DisplayerLocation (`KismetMathLibrary.MakeRotator` _returnvalue_roll 0.0 _returnvalue_yaw)) "AlwaysSpawn" "OverrideRootScale" null (`self.ShouldReplicates`) (`GameplayStatics.GetPlayerPawn` 0)))
      (bind _output_get (set `self.DisplayerActor` _returnvalue))
      (message `/Game/Blueprints/Interfaces/BPI_Displayer.ChangeText` _output_get TextToShow))))

(event `CreateDisplayer`
  (params (TextToShow :type Text) (DisplayerLocation :type "Vector Structure"))
  (if (`self.ShouldReplicates`)
    (`self.Server_CreateDisplayer` TextToShow DisplayerLocation)
    (`self.Multi_PlaySound`)
    (else
      (`self.Client_CreateDisplayer` TextToShow DisplayerLocation)
      (`GameplayStatics.PlaySound2D` (`self.SFX`) 1.0 1.0 0.0 null null))))

(event `Server_EditDisplayer`
  (params (TextToShow :type Text))
  (bind _displayeractor (`self.DisplayerActor`))
  (`/Engine/EditorBlueprintResources/StandardMacros.IsValid` _displayeractor
    (:`Is Valid`
      (message `/Game/Blueprints/Interfaces/BPI_Displayer.ChangeText` _displayeractor TextToShow))))

(event `Client_EditDisplayer`
  (params (TextToShow :type Text))
  (bind _displayeractor (`self.DisplayerActor`))
  (`/Engine/EditorBlueprintResources/StandardMacros.IsValid` _displayeractor
    (:`Is Valid`
      (message `/Game/Blueprints/Interfaces/BPI_Displayer.ChangeText` _displayeractor TextToShow))))

(event `EditDisplayer`
  (params (TextToShow :type Text))
  (if (`self.ShouldReplicates`)
    (`self.Server_EditDisplayer` TextToShow)
    (`self.Multi_PlaySound`)
    (else
      (`self.Client_EditDisplayer` TextToShow)
      (`GameplayStatics.PlaySound2D` (`self.SFX`) 1.0 1.0 0.0 null null))))

(event `DeleteDisplayer`
  (if (`self.ShouldReplicates`)
    (`self.Server_DeleteDisplayer`)
    (else
      (`self.Client_DeleteDisplayer`))))

(event `Server_DeleteDisplayer`
  (bind _existingdisplayer (`self.GetExistingDisplayer`))
  (`/Engine/EditorBlueprintResources/StandardMacros.IsValid` _existingdisplayer
    (:`Is Valid`
      (`Actor.K2_DestroyActor` _existingdisplayer))))

(event `Client_DeleteDisplayer`
  (bind _displayeractor (`self.DisplayerActor`))
  (`/Engine/EditorBlueprintResources/StandardMacros.IsValid` _displayeractor
    (:`Is Valid`
      (`Actor.K2_DestroyActor` _displayeractor))))

(event `Multi_PlaySound`
  (`GameplayStatics.PlaySound2D` (`self.SFX`) 1.0 1.0 0.0 null (`GameplayStatics.GetPlayerController` 0)))

(fn `GetExistingDisplayer`
  (returns (ExistingDisplayer :type "/Game/Blueprints/BP_Displayer Object Reference"))
  (bind _displayeractor (`self.DisplayerActor`))
  (`/Engine/EditorBlueprintResources/StandardMacros.IsValid` _displayeractor
    (:`Is Valid`
      (return _displayeractor))
    (:`Is Not Valid`
      (bind _returnvalue (`GameplayStatics.GetActorOfClass` (`self.DisplayerClass`)))
      (`/Engine/EditorBlueprintResources/StandardMacros.IsValid` _returnvalue
        (:`Is Valid`
          (return _returnvalue))
        (:`Is Not Valid`
          (return null))))))