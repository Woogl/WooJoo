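; BP_Displayer is a Blueprint that shows a changeable text message through a Widget component.
; The construction script sets actor replication from the ShouldReplicates flag.
; ChangeText uses the same flag to route the text to a Multi or Client event, named as multicast and client variants.
; Both events pass the text to ChangeTextMessage on the component's user widget.
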(event `/Game/Blueprints/Interfaces/BPI_Displayer.ChangeText`
  (params (TextToShow :type Text))
  (if (`self.ShouldReplicates`)
    (`self.Multi_ChangeText` TextToShow)
    (else
      (`self.Client_ChangeText` TextToShow))))

(event `Multi_ChangeText`
  (params (TextToShow :type Text))
  (message `/Game/Blueprints/Interfaces/BPI_Displayer.ChangeText` (`WidgetComponent.GetUserWidgetObject` (`self.Widget`)) TextToShow))

(event `Client_ChangeText`
  (params (TextToShow :type Text))
  (message `/Game/Blueprints/Interfaces/BPI_Displayer.ChangeText` (`WidgetComponent.GetUserWidgetObject` (`self.Widget`)) TextToShow))

(fn `UserConstructionScript`
  (`self.SetReplicates` (`self.ShouldReplicates`)))