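; PC player pawn for Woogle, with Enhanced Input movement and look, plus debug hooks for text displayers and menus.
; Move input follows control rotation and look input yaws the mesh; non-authority instances push location and mesh rotation through server events that teleport them.
; Number keys test creating and deleting displayers through local and multiplayer manager components.
; BeginPlay adds the input mapping, then TestUI opens the main or in-game menu by level name.
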(event `Key|One`
  (params (Key :type "Key Structure"))
  ;[1 1 1] Test Zone
  (:`Pressed`
    (`/Game/Blueprints/Components/BP_DisplayerManager.CreateDisplayer` (`self.BP_DisplayerManager_Local`) "Local 1" (125.0 0.0 25.0))))

(event `Key|Five`
  (params (Key :type "Key Structure"))
  ;[1 1 1] Test Zone
  (:`Pressed`
    (`/Game/Blueprints/Components/BP_DisplayerManager.DeleteDisplayer` (`self.BP_DisplayerManager_Local`))))

(event `Key|Two`
  (params (Key :type "Key Structure"))
  ;[1 1 1] Test Zone
  (:`Pressed`
    (`/Game/Blueprints/Components/BP_DisplayerManager.CreateDisplayer` (`self.BP_DisplayerManager_Local`) "Local 2" (125.0 0.0 25.0))))

(event `Key|Three`
  (params (Key :type "Key Structure"))
  ;[1 1 1] Test Zone
  (:`Pressed`
    (`/Game/Blueprints/Components/BP_DisplayerManager.Server_CreateDisplayer` (`self.BP_DisplayerManager_Multi`) "Multi 3" (125.0 0.0 150.0))))

(event `Key|Six`
  (params (Key :type "Key Structure"))
  ;[1 1 1] Test Zone
  (:`Pressed`
    (`/Game/Blueprints/Components/BP_DisplayerManager.Server_DeleteDisplayer` (`self.BP_DisplayerManager_Multi`))))

(event `self.ReceiveBeginPlay`
  ;[0 0 0] Setup
  (`EnhancedInputSubsystemInterface.AddMappingContext` (pcsubsystem `EnhancedInputLocalPlayerSubsystem` (`GameplayStatics.GetPlayerController` 0)) "/Game/Woogle/IMC_WooglePawn.IMC_WooglePawn" 0 (struct))
  ;;[1 1 1] UI Debug
  (`self.TestUI`))

(event `Key|Four`
  (params (Key :type "Key Structure"))
  ;[1 1 1] Test Zone
  (:`Pressed`
    (`/Game/Blueprints/Components/BP_DisplayerManager.Server_CreateDisplayer` (`self.BP_DisplayerManager_Multi`) "Multi 4" (125.0 0.0 150.0))))

(event `Server_SetLocation`
  (params (LocationToSend :type "Vector Structure"))
  ;[0 0 0] Replication
  (`self.K2_SetActorLocation` LocationToSend false true))

(event `EnhancedInput|/Game/Woogle/IA_WoogleMove`
  (params (ActionValue :type "Vector2D Structure") (ElapsedSeconds :type "Float (double-precision)") (TriggeredSeconds :type "Float (double-precision)") (InputAction :type "InputAction Object Reference" :default "/Game/Woogle/IA_WoogleMove.IA_WoogleMove"))
  (bind (_returnvalue_roll _returnvalue_pitch _returnvalue_yaw) (`KismetMathLibrary.BreakRotator` (`self.GetControlRotation`)))
  (bind (_returnvalue_roll_2 _returnvalue_pitch_2 _returnvalue_yaw_2) (`KismetMathLibrary.BreakRotator` (`self.GetControlRotation`)))
  ;[0 0 0] Inputs
  (:`Triggered`
    (`self.AddMovementInput` (`KismetMathLibrary.GetRightVector` (`KismetMathLibrary.MakeRotator` _returnvalue_roll_2 0.0 _returnvalue_yaw_2)) ActionValue_X)
    (`self.AddMovementInput` (`KismetMathLibrary.GetForwardVector` (`KismetMathLibrary.MakeRotator` 0.0 0.0 _returnvalue_yaw)) ActionValue_Y)
    (if (not (`self.HasAuthority`))
      (`self.Server_SetLocation` (`self.K2_GetActorLocation`)))))

(event `Server_SetMeshRotation`
  (params (RotationToSend :type "Rotator Structure"))
  ;[0 0 0] Replication
  (`SceneComponent.K2_SetWorldRotation` (`self.StaticMesh`) RotationToSend false true))

(event `EnhancedInput|/Game/Woogle/IA_WoogleLook`
  (params (ActionValue :type "Vector2D Structure") (ElapsedSeconds :type "Float (double-precision)") (TriggeredSeconds :type "Float (double-precision)") (InputAction :type "InputAction Object Reference" :default "/Game/Woogle/IA_WoogleLook.IA_WoogleLook"))
  (bind (_returnvalue_roll _returnvalue_pitch _returnvalue_yaw) (`KismetMathLibrary.BreakRotator` (`self.GetControlRotation`)))
  (bind _staticmesh (`self.StaticMesh`))
  ;[0 0 0] Inputs
  (:`Triggered`
    (`self.AddControllerYawInput` (* ActionValue_X -1))
    (`self.AddControllerPitchInput` ActionValue_Y)
    (`SceneComponent.K2_SetWorldRotation` _staticmesh (`KismetMathLibrary.MakeRotator` 0.0 0.0 _returnvalue_yaw) false false)
    (if (not (`self.HasAuthority`))
      (`self.Server_SetMEshRotation` (`SceneComponent.K2_GetComponentRotation` _staticmesh)))))

(fn `TestUI`
  (bind _returnvalue (`GameplayStatics.GetPlayerController` 0))
  (bind _returnvalue_2 (`GameplayStatics.GetPlayerController` 0))
  (bind _returnvalue_3 (`GameplayStatics.GetCurrentLevelName` true))
  (if (`KismetStringLibrary.EqualEqual_StrStr` _returnvalue_3 "LV_Main")
    (bind _returnvalue_4 (`|CreateWidget` "/Game/Blueprints/UI/WBP_MainMenu.WBP_MainMenu_C" _returnvalue_2))
    (`UserWidget.AddToViewport` _returnvalue_4 0)
    (set `PlayerController.bShowMouseCursor` true _returnvalue_2)
    (elif (or (`KismetStringLibrary.EqualEqual_StrStr` _returnvalue_3 "LV_BoardGame") (`KismetStringLibrary.EqualEqual_StrStr` "LV_Counsel" _returnvalue_3))
      (bind _returnvalue_5 (`|CreateWidget` "/Game/Blueprints/UI/WBP_InGameMenu.WBP_InGameMenu_C" _returnvalue))
      (`UserWidget.AddToViewport` _returnvalue_5 0)
      (set `PlayerController.bShowMouseCursor` true _returnvalue))))

(fn `UserConstructionScript`)