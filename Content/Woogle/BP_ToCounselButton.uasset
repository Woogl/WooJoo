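; BP_ToCounselButton is an interactable button that sends players to the LV_Counsel map and shows a text displayer at its location.
; On interact with one player or no valid GameMode, it creates an advanced session tagged with host name and counsel mode, then opens the map.
; Otherwise it runs a ServerTravel console command to that map.
; The session's UseLAN flag is true when the Steam subsystem is present.
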(event `self.ReceiveBeginPlay`
  (`/Game/Blueprints/Components/BP_DisplayerManager.CreateDisplayer` (`self.BP_DisplayerManager`) (`self.Text to Show`) (`self.K2_GetActorLocation`)))

(event `/Game/Blueprints/Interfaces/BPI_Interact.Interact`
  (bind _returnvalue (`GameplayStatics.GetGameMode`))
  (`/Engine/EditorBlueprintResources/StandardMacros.IsValid` _returnvalue
    (:`Is Valid`
      (bind _returnvalue_2 (`GameModeBase.GetNumPlayers` _returnvalue))
      (if (== _returnvalue_2 1)
        (`self.CreateNewSession` :!label _label)
        (else
          (`KismetSystemLibrary.ExecuteConsoleCommand` "ServerTravel /Game/Maps/LV_Counsel" null))))
    (:`Is Not Valid`
      (goto _label))))

(event `CreateNewSession`
  (`CreateSessionCallbackProxyAdvanced.CreateAdvancedSession` (`|MakeArray` (`AdvancedSessionsLibrary.MakeLiteralSessionPropertyString` "HostNameKey" (`AdvancedSessionsLibrary.GetPlayerName` (`GameplayStatics.GetPlayerController` 0))) (`AdvancedSessionsLibrary.MakeLiteralSessionPropertyBool` "CounselModeKey" true)) (`GameplayStatics.GetPlayerController` 0) (`self.MaxPlayers`) 0 (`AdvancedSessionsLibrary.HasOnlineSubsystem` "Steam")
    (:`OnSuccess`
      (`GameplayStatics.OpenLevel` "LV_Counsel"))))

(fn `UserConstructionScript`)