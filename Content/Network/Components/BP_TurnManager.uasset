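; Network turn component for the WooJoo board game that tracks whether it is this player's turn and shows that status.
; It adds two DisplayerManagers to its owner, one for turn text and one for the pre-game countdown, which ends by calling StartBoardGame on the game mode.
; Turn events toggle IsMyTurn and the label.
; Test keys drive the game mode: Space requests turn cycling through a server action on the player's turn, Enter calls LetsStart.
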(event `self.ReceiveBeginPlay`
  ;[0 0 0] Setup
  (bind _returnvalue (`|AddComponentByClass` (`self.GetOwner`) "/Game/Network/Components/BP_DisplayerManager.BP_DisplayerManager_C" null))
  (set `self.DisplayerManager_Ruler` _returnvalue)
  (bind _returnvalue_2 (`|AddComponentByClass` (`self.GetOwner`) "/Game/Network/Components/BP_DisplayerManager.BP_DisplayerManager_C" null))
  (set `self.DisplayerManager_Countdown` _returnvalue_2))

(event `Server_Action`
  (bind _asbp_woo_joo_game_mode (cast `/Game/Network/Blueprints/BP_WooJooGameMode` (`GameplayStatics.GetGameMode`)))
  (`/Game/Network/Blueprints/BP_WooJooGameMode.CycleTurns` _asbp_woo_joo_game_mode))

(event `OnStartBoardGame`
  (if (`Controller.IsLocalController` (`GameplayStatics.GetPlayerController` 0))
    (`/Game/Network/Components/BP_DisplayerManager.CreateDisplayer` (`self.DisplayerManager_Ruler`) (select `bool` (`self.IsMyTurn`) :`false` "WAITING" :`true` "YOUR TURN" :!type "Text") (`self.GetRightUIPosition` (125.0 0.0 100.0)))))

(event `Key|SpaceBar`
  (params (Key :type "Key Structure"))
  ;[1 1 1] Input Test
  (:`Pressed`
    (if (`self.IsMyTurn`)
      (`self.HandleSpaceBar`))))

(event `Key|Enter`
  (params (Key :type "Key Structure"))
  ;[1 1 1] Input Test
  (:`Pressed`
    (bind _asbp_woo_joo_game_mode (cast `/Game/Network/Blueprints/BP_WooJooGameMode` (`GameplayStatics.GetGameMode`)))
    (`/Game/Network/Blueprints/BP_WooJooGameMode.LetsStart` _asbp_woo_joo_game_mode)))

(event `OnStartTurn`
  (set `self.IsMyTurn` true)
  (`/Game/Network/Components/BP_DisplayerManager.EditDisplayer` (`self.DisplayerManager_Ruler`) "YOUR TURN"))

(event `OnEndTurn`
  (set `self.IsMyTurn` false)
  (`/Game/Network/Components/BP_DisplayerManager.EditDisplayer` (`self.DisplayerManager_Ruler`) "WAITING"))

(event `OnCountdown`
  (`/Game/Network/Components/BP_DisplayerManager.CreateDisplayer` (`self.DisplayerManager_Countdown`) "Ready to Start Game !" (125.0 0.0 200.0))
  (`KismetSystemLibrary.Delay` 2.0)
  (`/Game/Network/Components/BP_DisplayerManager.CreateDisplayer` (`self.DisplayerManager_Countdown`) "3" (125.0 0.0 200.0))
  (`KismetSystemLibrary.Delay` 1.0)
  (`/Game/Network/Components/BP_DisplayerManager.CreateDisplayer` (`self.DisplayerManager_Countdown`) "2" (125.0 0.0 200.0))
  (`KismetSystemLibrary.Delay` 1.0)
  (`/Game/Network/Components/BP_DisplayerManager.CreateDisplayer` (`self.DisplayerManager_Countdown`) "1" (125.0 0.0 200.0))
  (`KismetSystemLibrary.Delay` 1.0)
  (`/Game/Network/Components/BP_DisplayerManager.CreateDisplayer` (`self.DisplayerManager_Countdown`) "Game Start !" (125.0 0.0 200.0))
  (`KismetSystemLibrary.Delay` 2.0)
  (`/Game/Network/Components/BP_DisplayerManager.DeleteDisplayer` (`self.DisplayerManager_Countdown`))
  (bind _asbp_woo_joo_game_mode (cast `/Game/Network/Blueprints/BP_WooJooGameMode` (`GameplayStatics.GetGameMode`)))
  (`/Game/Network/Blueprints/BP_WooJooGameMode.StartBoardGame` _asbp_woo_joo_game_mode))

(fn `HandleSpaceBar`
  (`self.Server_Action`))