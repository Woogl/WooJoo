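; BP_DisplayerManager is a network component that creates, edits and deletes a text displayer actor.
; Each action has a Server event that calls a Multi event, which runs the local logic.
; Creation reuses the stored DisplayerActor by teleporting it and changing its text, or spawns one from DisplayerClass if none is valid.
; Creating or editing also plays a 2D sound, while deletion destroys the actor.
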(event `Server_CreateDisplayer`
  (params (TextToShow :type Text) (`Spawn Transform Location` :type "Vector Structure"))
  (`self.Multi_CreateDisplayer` TextToShow `Spawn Transform Location`))

(event `Multi_CreateDisplayer`
  (params (TextToShow :type Text) (DisplayerLocation :type "Vector Structure"))
  (`self.CreateDisplayer` TextToShow DisplayerLocation))

(event `CreateDisplayer`
  (params (TextToShow :type Text) (DisplayerLocation :type "Vector Structure"))
  (`/Engine/EditorBlueprintResources/StandardMacros.IsValid` (`self.DisplayerActor`)
    (:`Is Valid`
      (`Actor.K2_SetActorLocation` (`self.DisplayerActor`) DisplayerLocation false true)
      (message `/Game/Network/Interfaces/BPI_Displayer.ChangeText` (`self.DisplayerActor`) TextToShow))
    (:`Is Not Valid`
      (bind _returnvalue (`|SpawnActorFromClass` (`self.DisplayerClass`) (`KismetMathLibrary.MakeTransform` DisplayerLocation) "AlwaysSpawn" "OverrideRootScale" null (`GameplayStatics.GetPlayerPawn` 0)))
      (bind _output_get (set `self.DisplayerActor` _returnvalue))
      (message `/Game/Network/Interfaces/BPI_Displayer.ChangeText` _output_get TextToShow)))
  (`GameplayStatics.PlaySound2D` (`self.SFX`) 1.0 1.0 0.0 null null))

(event `Server_EditDisplayer`
  (params (TextToShow :type Text))
  (`self.Multi_EditDisplayer` TextToShow))

(event `Multi_EditDisplayer`
  (params (TextToShow :type Text))
  (`self.EditDisplayer` TextToShow))

(event `EditDisplayer`
  (params (TextToShow :type Text))
  (bind _displayeractor (`self.DisplayerActor`))
  (`/Engine/EditorBlueprintResources/StandardMacros.IsValid` _displayeractor
    (:`Is Valid`
      (message `/Game/Network/Interfaces/BPI_Displayer.ChangeText` _displayeractor TextToShow)
      (`GameplayStatics.PlaySound2D` (`self.SFX`) 1.0 1.0 0.0 null null))))

(event `Server_DeleteDisplayer`
  (`self.Multi_DeleteDisplayer`))

(event `Multi_DeleteDisplayer`
  (`self.DeleteDisplayer`))

(event `DeleteDisplayer`
  (bind _displayeractor (`self.DisplayerActor`))
  (`/Engine/EditorBlueprintResources/StandardMacros.IsValid` _displayeractor
    (:`Is Valid`
      (`Actor.K2_DestroyActor` _displayeractor))))