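; BP_SessionPlanet is an actor that represents a found online session as a planet that can be entered to join it.
; On BeginPlay it reads SessionInfo and its extra settings to label three text renders with host name, mode (Counseling or Board Game) and player count.
; Any overlap with its Sphere calls JoinSession on that result for player controller 0, without filtering the overlapping actor.
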(event `self.ReceiveBeginPlay`
  (bind _sessioninfo (`self.SessionInfo`))
  (bind _extrasettings (`AdvancedSessionsLibrary.GetExtraSettings` (`self.SessionInfo`)))
  (`|ExecutionSequence`
    (:`then_0`
      (bind _settingvalue (`AdvancedSessionsLibrary.GetSessionPropertyString` _extrasettings "HostNameKey")
        (:`Found`
          (`TextRenderComponent.K2_SetText` (`self.TextRender`) (`|FormatText` "{Name}'s Planet" (`KismetTextLibrary.Conv_StringToText` _settingvalue))))))
    (:`then_1`
      (bind _settingvalue_2 (`AdvancedSessionsLibrary.GetSessionPropertyBool` _extrasettings "CounselModeKey")
        (:`Found`
          (`TextRenderComponent.K2_SetText` (`self.TextRender1`) (select `bool` _settingvalue_2 :`false` "Board Game" :`true` "Counseling")))))
    (:`then_2`
      (`TextRenderComponent.K2_SetText` (`self.TextRender2`) (`|FormatText` "{Cur} / {Max}" (`FindSessionsCallbackProxy.GetCurrentPlayers` _sessioninfo) (`FindSessionsCallbackProxy.GetMaxPlayers` _sessioninfo))))))

(event `self.Sphere.OnComponentBeginOverlap`
  (params (OverlappedComponent :type "PrimitiveComponent Object Reference") (OtherActor :type "Actor Object Reference") (OtherComp :type "PrimitiveComponent Object Reference") (OtherBodyIndex :type Integer) (bFromSweep :type Boolean) (SweepResult :type "HitResult Structure (by ref)"))
  (`KismetSystemLibrary.PrintString` "Session Planet Overlap")
  (`JoinSessionCallbackProxy.JoinSession` (`GameplayStatics.GetPlayerController` 0) (`self.SessionInfo`)))

(fn `UserConstructionScript`)