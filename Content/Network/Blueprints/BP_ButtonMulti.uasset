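; Interactable button that plays a sound and starts a multiplayer game on the multiplayer map.
; With authority, it server-travels to LV_Multi and updates the session; otherwise it creates an advanced session and opens the level as a listen server on success.
; Both paths publish host name and a disabled counsel-mode flag, cap connections at MaxPlayers, and set LAN use from the Steam subsystem check.
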(event `/Game/Network/Interfaces/BPI_Interact.Interact`
  (`GameplayStatics.PlaySound2D` (`self.Sound`) 1.0 1.0 0.0 null null)
  (`/Engine/EditorBlueprintResources/ActorMacros.Switch Has Authority`
    (:`Authority`
      (`KismetSystemLibrary.ExecuteConsoleCommand` "ServerTravel /Game/Maps/LV_Multi" null)
      (`UpdateSessionCallbackProxyAdvanced.UpdateSession` (`|MakeArray` (`AdvancedSessionsLibrary.MakeLiteralSessionPropertyString` "HostNameKey" (`AdvancedSessionsLibrary.GetPlayerName` (`GameplayStatics.GetPlayerController` 0))) (`AdvancedSessionsLibrary.MakeLiteralSessionPropertyBool` "CounselModeKey")) (`self.MaxPlayers`) 0 (`AdvancedSessionsLibrary.HasOnlineSubsystem` "Steam") true true))
    (:`Remote`
      (`self.CreateNewSession`))))

(event `CreateNewSession`
  (`CreateSessionCallbackProxyAdvanced.CreateAdvancedSession` (`|MakeArray` (`AdvancedSessionsLibrary.MakeLiteralSessionPropertyString` "HostNameKey" (`AdvancedSessionsLibrary.GetPlayerName` (`GameplayStatics.GetPlayerController` 0))) (`AdvancedSessionsLibrary.MakeLiteralSessionPropertyBool` "CounselModeKey")) (`GameplayStatics.GetPlayerController` 0) (`self.MaxPlayers`) 0 (`AdvancedSessionsLibrary.HasOnlineSubsystem` "Steam")
    (:`OnSuccess`
      (`GameplayStatics.OpenLevelBySoftObjectPtr` (`self.MultiLevel`) true "listen"))))

(fn `UserConstructionScript`
  (`parent.UserConstructionScript`))