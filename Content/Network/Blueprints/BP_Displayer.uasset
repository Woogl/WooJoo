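; BP_Displayer is an actor that shows a text message on a widget and keeps it turned toward the local player.
; Each tick it rotates to look at the first player pawn's camera component, falling back to the pawn's location when no camera exists.
; The construction script applies the default text, and a ChangeText event passes new messages to the widget at runtime.
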(event `self.ReceiveTick`
  (params (DeltaSeconds :type "Float (single-precision)"))
  (bind _returnvalue (`GameplayStatics.GetPlayerPawn` 0))
  (bind _returnvalue_2 (`self.GetComponentByClass` (`GameplayStatics.GetPlayerPawn` 0) "/Script/Engine.CameraComponent"))
  (`/Engine/EditorBlueprintResources/StandardMacros.IsValid` _returnvalue_2
    (:`Is Valid`
      (`self.K2_SetActorRotation` (`KismetMathLibrary.FindLookAtRotation` (`self.K2_GetActorLocation`) (`SceneComponent.K2_GetComponentLocation` _returnvalue_2))))
    (:`Is Not Valid`
      (`/Engine/EditorBlueprintResources/StandardMacros.IsValid` _returnvalue
        (:`Is Valid`
          (`self.K2_SetActorRotation` (`KismetMathLibrary.FindLookAtRotation` (`self.K2_GetActorLocation`) (`self.K2_GetActorLocation` _returnvalue))))))))

(event `/Game/Network/Interfaces/BPI_Displayer.ChangeText`
  (params (TextToShow :type Text))
  (message `/Game/Network/Interfaces/BPI_Displayer.ChangeText` (`WidgetComponent.GetUserWidgetObject` (`self.Widget`)) TextToShow))

(fn `UserConstructionScript`
  (message `/Game/Network/Interfaces/BPI_Displayer.ChangeText` (`self.Widget`) (`self.DefaultText`)))